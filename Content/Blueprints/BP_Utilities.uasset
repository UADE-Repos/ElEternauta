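; BP_Utilities is a utility Blueprint with one function, GetPointInRadious, which returns a random point around an input vector on the same Z.
; It offsets X and Y by cosine and sine of random angles, scaled by random distances up to MaxSpawnRadious.
; Each axis draws its own angle and distance, so results are non-uniform and can fall outside the circle, within its bounding square.
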(fn GetPointinRadious
  (params (InVec :type Vector) (MaxSpawnRadious :type Float%20%28double-precision%29))
  (bind (_x _y _z) (Math|Vector|BreakVector InVec))
  (bind _returnvalue (Math|Random|RandomFloatinRange 0.0 MaxSpawnRadious))
  (bind _returnvalue_2 (Math|Random|RandomFloatinRange 0.0 359.0))
  (return (Math|Vector|MakeVector (+ (* (Math|Trig|Cos(Degrees) _returnvalue_2) _returnvalue) _x) (+ (* (Math|Trig|Sin(Degrees) _returnvalue_2) _returnvalue) _y) _z)))