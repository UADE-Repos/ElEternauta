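; A dropped-object actor that takes its static mesh from a variable and flies to the player when interacted with.
; On BeginPlay it applies the mesh, then disables collision and re-enables it after a brief timer.
; InteractionResult stops physics, then a timeline lerps the actor from its current spot to the passed actor's live location and destroys it on finish.
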(event Custom|ReEnableCollision
  (Collision|SetActorEnableCollision true))

(event EventBeginPlay
  (bind _mesh (Variables|Default|GetMesh))
  (Utilities|IsValid _mesh
    (:Is%20Valid
      (Components|StaticMesh|SetStaticMesh (Variables|Default|GetStaticMesh) _mesh)
      (Collision|SetActorEnableCollision false)
      (Utilities|Time|SetTimerbyEvent (delegate Custom|ReEnableCollision) 0.05))))

(event EventInteractionResult
  (params (PlayerPosition :type Actor%20Object%20Reference))
  (Physics|SetSimulatePhysics (Variables|Default|GetStaticMesh) false)
  (bind _output_get (Variables|Default|SetTempLocation (Transformation|GetActorLocation)))
  (bind _gotoplayer (Timeline|GoToPlayer PlayFromStart)
    (:Update
      (Transformation|SetActorLocation (Math|Vector|Lerp(Vector) _output_get (Transformation|GetActorLocation PlayerPosition) _gotoplayer) false false))
    (:Finished
      (Actor|DestroyActor))))

(fn ConstructionScript)