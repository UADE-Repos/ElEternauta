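; BP_TheSnowGathering tracks the player's gathered resources against required amounts for what appears to be a snow gathering objective.
; GatheredResource increments the count for types already in the Resource map, then runs CheckAmount.
; CheckAmount compares Resource and ResourceRequired values by array index, so both maps depend on matching key order.
; When every requirement is met, it prints a debug message and calls PlayerGotResources through a DoOnce.
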(event Custom|CheckAmount
  (Variables|Default|SetSucceded true)
  (bind _values (Utilities|Map|Values (Variables|Default|GetResourceRequired)))
  (bind _values_2 (Utilities|Map|Values (Variables|Default|GetResource)))
  (for (_array_element _array_index) _values
    (Math|Integer|CompareInt (Utilities|Array|Get(acopy) _values_2 _array_index) _array_element
      (:>
        (Variables|Default|SetTempSucceded true :!label _label))
      (:==
        (goto _label))
      (:<
        (Variables|Default|SetTempSucceded false)))
    (if (not (Variables|Default|GetTempSucceded))
      (Variables|Default|SetSucceded false)))
  (if (Variables|Default|GetSucceded)
    (Development|PrintString (Utilities|String|ToString(Boolean) (Variables|Default|GetSucceded)) true true "(R=0.323005,G=1.000000,B=0.000000,A=1.000000)" 1e+01)
    (Utilities|FlowControl|DoOnce false
      (:Completed
        (Default|CallPlayerGotResources)))))

(event EventBeginPlay
  (|CallParentFunction) ; This node is disabled and will not be called.\nDrag off pins to build functionality.
)

(event EventTick
  (params (DeltaSeconds :type Float%20%28single-precision%29)))

(event EventGatheredResource
  (params (Type :type E_ObjectType%20Enum :default "NewEnumerator0"))
  (bind _resource (Variables|Default|GetResource))
  (bind (_value _returnvalue) (Utilities|Map|Find _resource Type))
  (if _returnvalue
    (bind _result (Math|Integer|IncrementInt _value)
      (:%20%20
        (Utilities|Map|Add _resource Type _result)
        (CallFunction|CheckAmount)))))

(fn ConstructionScript
  (|CallParentFunction))