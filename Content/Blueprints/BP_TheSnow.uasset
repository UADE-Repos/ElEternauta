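; BP_TheSnow is a setup Blueprint that starts controllers and handles player death and level restarting.
; On BeginPlay it spawns BP_FogController and BP_WindowsController at the world origin, then finds BP_FirstPersonCharacter and binds an event to its death.
; RestartLevel, the apparent handler for that death, reopens the current level by name.
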(event Custom|RestartLevel
  (bind _returnvalue (Game|GetCurrentLevelName true))
  (Game|OpenLevel(byName) (Utilities|String|StringToName _returnvalue)))

(event EventBeginPlay
  (bind _returnvalue (Math|Transform|MakeTransform "0, 0, 0"))
  (Utilities|FlowControl|Sequence
    (:then_0
      (Game|SpawnActorfromClass "/Game/Blueprints/Controllers/BP_FogController.BP_FogController_C" _returnvalue "Undefined" "MultiplyWithRoot" 0 0))
    (:then_1
      (Game|SpawnActorfromClass "/Game/Blueprints/Controllers/BP_WindowsController.BP_WindowsController_C" _returnvalue "Undefined" "MultiplyWithRoot" 0 0))
    (:then_2
      (bind _returnvalue_2 (Actor|GetActorOfClass "/Game/Blueprints/BP_FirstPersonCharacter.BP_FirstPersonCharacter_C"))
      (bind _output_get (Variables|Default|SetPlayer _returnvalue_2))
      (EventDispatchers|BindEventtoPlayerDeath _output_get (EventDispatchers|CreateEvent :!event Custom|RestartLevel)))))

(fn ConstructionScript)