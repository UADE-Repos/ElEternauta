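; BP_ToolBox is an interactable toolbox pickup that grants the player an object disassembly component (AC_ObjectDissassemble).
; On BeginPlay, if a Mesh is set, it applies it to the StaticMesh and briefly toggles actor collision off, re-enabling it on a short timer.
; Interaction passes the player to GoToPlayerEvent, while OnPickUp adds the component to the player and destroys the toolbox.
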(event Custom|ReEnableCollision
  (Collision|SetActorEnableCollision true))

(event EventBeginPlay
  (bind _mesh (Variables|Default|GetMesh))
  (Utilities|IsValid _mesh
    (:Is%20Valid
      (Components|StaticMesh|SetStaticMesh (Variables|Default|GetStaticMesh) _mesh)
      (Collision|SetActorEnableCollision false)
      (Utilities|Time|SetTimerbyEvent (delegate Custom|ReEnableCollision) 0.05))))

(event EventInteractionResult
  (params (Player :type Actor%20Object%20Reference))
  (CallFunction|GotoPlayerEvent Player))

(event EventOnPickUp
  (Game|AddComponentbyClass (stale EventInteractionResult Player) "/Game/Blueprints/ActorComponents/AC_ObjectDissassemble.AC_ObjectDissassemble_C")
  (Actor|DestroyActor))

(fn ConstructionScript
  (|CallParentFunction))