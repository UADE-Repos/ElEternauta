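; Interactable world object that a player can disassemble into dropped objects when they have an AC_ObjectDissassemble component.
; Hovering caches whether the player has that component, which controls both the prompt text and whether interaction is allowed.
; On interaction it passes its disassemblable type and bounds center to the component's spawn message, then destroys itself.
; Its interaction time is zero.
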(event EventDoInteractionResult
  (params (HitResult :type Hit%20Result%20Structure) (Player :type Actor%20Object%20Reference))
  (bind _returnvalue (Actor|GetComponentbyClass Player "/Game/Blueprints/ActorComponents/AC_ObjectDissassemble.AC_ObjectDissassemble_C"))
  (Utilities|IsValid _returnvalue
    (:Is%20Valid
      (Class|BPISpawnerInterface|SpawnDroppedObjects(Message) _returnvalue (Variables|Default|GetDisassemblableType) (.Origin (Collision|GetActorBounds false false)))
      (Actor|DestroyActor))))

(fn ConstructionScript)

(fn CanbeInteracted
  (return (Variables|Default|GetHasToolbox?)))

(fn GetTime
  (return 0.0))

(fn IsHoveringActor
  (params (Hit :type Hit%20Result%20Structure) (Player :type Actor%20Object%20Reference))
  (bind _output_get (Variables|Default|SetHasToolbox? (Utilities|IsValid (Actor|GetComponentbyClass Player "/Game/Blueprints/ActorComponents/AC_ObjectDissassemble.AC_ObjectDissassemble_C"))))
  (if _output_get
    (return "Dissasemble?")
    (else
      (return ""))))