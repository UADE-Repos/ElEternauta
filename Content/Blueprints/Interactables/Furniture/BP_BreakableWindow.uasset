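; Breakable window interactable that can be shattered and then repaired through interaction.
; StartDestruction has the ACBreakMesh component swap in a broken mesh with a Niagara effect, spawn a damaging zone and flag the window broken.
; Interaction is offered only while broken, showing a "Repair?" prompt and supplying a repair time, then restores a fixed mesh.
; Both state changes fire broken or repaired notifications.
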(event Custom|StartDestruction
  (if (not (Variables|Default|GetAlreadyBroken?))
    (bind _returnvalue (Default|BreakItem (Variables|Default|GetAC_BreakMesh) (Variables|Default|GetBrokenMeshes) (Variables|Default|GetStaticMesh) (Variables|Default|GetEmitter%20to%20Spawn) self))
    (Default|SpawnDamagingZone (Variables|Default|GetAC_BreakMesh) self (Variables|Default|GetDamageBoxOffsetLocation) (Variables|Default|GetDamageBoxScale) _returnvalue)
    (Variables|Default|SetAlreadyBroken? true)
    (Default|CallWindowHasBroken self)))

(event EventDoInteractionResult
  (params (HitResult :type Hit%20Result%20Structure) (Player :type Actor%20Object%20Reference))
  (if (Variables|Default|GetAlreadyBroken?)
    (Default|Repair? (Variables|Default|GetAC_BreakMesh) (Variables|Default|GetStaticMesh) (Variables|Default|GetFixedMeshes))
    (Default|CallWindowHasRepaired self)
    (Variables|Default|SetAlreadyBroken? false)))

(fn ConstructionScript)

(fn CanbeInteracted
  (return (Variables|Default|GetAlreadyBroken?)))

(fn GetTime
  (return (Variables|Default|GetTimeToRepair)))

(fn IsHoveringActor
  (params (Hit :type Hit%20Result%20Structure) (Player :type Actor%20Object%20Reference))
  (if (Variables|Default|GetAlreadyBroken?)
    (return "Repair?")
    (else
      (return ""))))