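; BP_Resource is a pickup interactable representing a gatherable resource of a configurable type.
; On pickup it runs the parent logic, then reports the resource type to the game mode through BPI_PlayerGatheredResource, if that interface is implemented.
; It is always interactable with a zero interaction time, shows a "Pick Up" hover prompt naming the type, and applies its configured mesh at BeginPlay.
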(event EventOnPickUp
  (bind _returnvalue (Game|GetGameMode))
  (|CallParentFunction)
  (if (Utilities|DoesObjectImplementInterface _returnvalue "/Game/Blueprints/Interfaces/BPI_PlayerGatheredResource.BPI_PlayerGatheredResource_C")
    (Class|BPIPlayerGatheredResource|GatheredResource(Message) _returnvalue (Variables|Default|GetTypeOfResource))))

(event EventBeginPlay
  (Components|StaticMesh|SetStaticMesh (Variables|Default|GetStaticMesh) (Variables|Default|GetMesh)))

(fn ConstructionScript
  (|CallParentFunction))

(fn CanbeInteracted
  (return true))

(fn GetTime
  (return 0.0))

(fn IsHoveringActor
  (params (Hit :type Hit%20Result%20Structure) (Player :type Actor%20Object%20Reference))
  (return (Utilities|Text|ToText(String) (Utilities|String|Append "Pick Up " (Utilities|String|EnumtoString (Variables|Default|GetTypeOfResource)) " ?"))))