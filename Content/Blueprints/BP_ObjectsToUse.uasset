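; BP_ObjectsToUse is an interactable pickup actor that flies to the player and disappears when used.
; On interaction it disables physics on its static mesh and runs a timeline that lerps its location from its start point toward the player's current position.
; When the timeline finishes, it calls OnPickUp, which destroys the actor.
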(event Custom|GoToPlayerEvent
  (params (Target :type Actor%20Object%20Reference))
  ;[0.15 0.15 0.15 0.5] Go to Player On Interaction
  (Physics|SetSimulatePhysics (Variables|Default|GetStaticMesh) false)
  (bind _output_get (Variables|Default|SetTempLocation (Transformation|GetActorLocation)))
  (bind _gotoplayer (Timeline|Timeline PlayFromStart)
    (:Update
      (Transformation|SetActorLocation (Math|Vector|Lerp(Vector) _output_get (Transformation|GetActorLocation Target) _gotoplayer) false false))
    (:Finished
      (CallFunction|OnPickUp))))

(event Custom|OnPickUp
  ;[0.15 0.15 0.15 0.5] Event to Happen On Pick Up
  (Actor|DestroyActor))

(event EventInteractionResult
  (params (Player :type Actor%20Object%20Reference))
  ;[0.15 0.15 0.15 0.5] Interaction
  (CallFunction|GotoPlayerEvent Player))

(fn ConstructionScript)