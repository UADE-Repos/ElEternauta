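; An umbrella mesh component that the first-person player toggles to shield against a damage type, apparently snow.
; On BeginPlay it adds its input mapping context and snaps to the character's ToolSocket with the morph target closed.
; The toggle FlipFlops open and closed, opening only if no other tool is in use, and swaps the morph target.
; Through owner interface calls, opening grants invulnerability and stops damage; closing removes it and restarts damage if outside.
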(event Input|EnhancedActionEvents|EnhancedInputActionIA_UmbrellaToggle
  (params (ActionValue :type Boolean) (ElapsedSeconds :type Float%20%28double-precision%29) (TriggeredSeconds :type Float%20%28double-precision%29) (InputAction :type Input%20Action%20Object%20Reference :default "/Game/Input/Actions/IA_UmbrellaToggle.IA_UmbrellaToggle"))
  (bind _owner (Variables|Default|GetOwner))
  (bind _owner_2 (Variables|Default|GetOwner))
  (bind _typeofinvulneravility (Variables|Default|GetTypeOfInvulneravility))
  (if (Utilities|DoesObjectImplementInterface _owner "/Game/Blueprints/Interfaces/BPI_SnowDamage.BPI_SnowDamage_C")
    (if (Variables|Default|GetBeingUsed?)
      (bind _isa (Utilities|FlowControl|FlipFlop :!label _label)
        (:A
          (Variables|Default|SetBeingUsed? _isa)
          (Class|BPITools|UsingTool(Message) (Variables|Default|GetOwner) _isa)
          (Audio|PlaySound2D "/Game/Sounds/AssetsSounds/UmbrellaOpen.UmbrellaOpen" 1.0 1.0 0.0 0 0)
          (Class|BPISnowDamage|StopDamagewithType(Message) _owner_2 _typeofinvulneravility)
          (Class|BPISnowDamage|AddInvulnerability(Message) _owner_2 _typeofinvulneravility)
          (Development|PrintString "UmbrellaOpen")
          (Components|SkeletalMesh|SetMorphTarget "UmbrellaOpenClosed" 0.0 true))
        (:B
          (Variables|Default|SetBeingUsed? _isa)
          (Class|BPITools|UsingTool(Message) (Variables|Default|GetOwner) _isa)
          (Audio|PlaySound2D "/Game/Sounds/AssetsSounds/UmbrellaOpen.UmbrellaOpen" 1.0 1.0 0.0 0 0)
          (Utilities|FlowControl|Sequence
            (:then_0
              (Class|BPISnowDamage|RemoveInvulnerability(Message) (Variables|Default|GetOwner) (Variables|Default|GetTypeOfInvulneravility))
              (Development|PrintString "UmbrellaClosed")
              (Components|SkeletalMesh|SetMorphTarget "UmbrellaOpenClosed" 1.0 true))
            (:then_1
              (bind _playeroutside_ (Class|BPISnowDamage|IsPlayerOutside?(Message) (Variables|Default|GetOwner)))
              (if _playeroutside_
                (Class|BPISnowDamage|StartDamagingwithType(Message) (Variables|Default|GetOwner) (Variables|Default|GetTypeOfInvulneravility)))))))
      (else
        (bind _condition_ (Class|BPITools|IsUsingTool?(Message) _owner))
        (if (not _condition_)
          (goto _label))))))

(event EventBeginPlay
  (Input|AddMappingContext (PlayerController|LocalPlayerSubsystems|GetEnhancedInputLocalPlayerSubsystem (Game|GetPlayerController 0)) "/Game/Input/IMC_Umbrella.IMC_Umbrella" 0 "(bIgnoreAllPressedKeysUntilRelease=True,bForceImmediately=False,bNotifyUserSettings=False)")
  (bind _output_get (Variables|Default|SetOwner (Components|GetOwner)))
  (bind _asbp_first_person_character (Utilities|Casting|CastToBP_FirstPersonCharacter _output_get))
  (Transformation|AttachComponentToComponent (Variables|/Game/Blueprints/BP_FirstPersonCharacter.BP_FirstPersonCharacter_C|GetFirstPersonMesh _asbp_first_person_character) "ToolSocket" "SnapToTarget" "SnapToTarget" "SnapToTarget" true)
  (Components|SkeletalMesh|SetMorphTarget "UmbrellaOpenClosed" 1.0 true))