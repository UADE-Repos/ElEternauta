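; Actor component that spawns dropped BP_Resource actors when an object is disassembled.
; SpawnDroppedObjects turns the disassemble type enum into a row name and looks it up in DTDisassembleObjects.
; The row's parallel type, mesh and quantity arrays set what spawns and how many, each placed at a GetPointInRadious location around the spawn point within MaxSpawnRadious.
; BeginPlay also fetches the table's row names, though spawning does not use them.
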(event EventBeginPlay
  (bind _outrownames (DataTable|GetDataTableRowNames (Variables|Default|GetDT_DisassembleObjects)))
  (Variables|Default|SetOut%20Row%20Names _outrownames))

(event EventSpawnDroppedObjects
  (params (TypeOfDisassemble :type E_DisassemblableType%20Enum :default "NewEnumerator7") (SpawnLocation :type Vector :default "0, 0, 0"))
  (bind _returnvalue (Utilities|GetDataTableRow (Variables|Default|GetDT_DisassembleObjects) (Utilities|String|StringToName (Utilities|String|EnumtoString TypeOfDisassemble)))
    (:then
      (for (_array_element _array_index) (.ObjectTypes (Utilities|Struct|BreakS_ItemToDrop _returnvalue))
        (Variables|Default|SetCurrentType _array_element)
        (Variables|Default|SetCurrentMesh (Utilities|Array|Get(acopy) (.ObjectMesh (Utilities|Struct|BreakS_ItemToDrop _returnvalue)) _array_index))
        (for _index (range 0 (- (Utilities|Array|Get(acopy) (.Quantities (Utilities|Struct|BreakS_ItemToDrop _returnvalue)) _array_index) 1))
          (Development|PrintString (Utilities|String|ToString(Integer) _index))
          (Game|SpawnActorfromClass "/Game/Blueprints/Interactables/Tools/BP_Resource.BP_Resource_C" (Math|Transform|MakeTransform (CallFunction|GetPointinRadious SpawnLocation (Variables|Default|GetMax%20Spawn%20Radious))) "AlwaysSpawn" "MultiplyWithRoot" 0 (Variables|Default|GetCurrentType) (Variables|Default|GetCurrentMesh) 0))))
    (:RowNotFound
      (Development|PrintString "Row Not Found"))))