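; AC_BreakMesh is an actor component that breaks and repairs static mesh items by swapping their meshes.
; BreakItem sets a replacement mesh, picked at random when several are supplied, then attaches an inactive Niagara system to the actor's root.
; SpawnDamagingZone separately spawns a BPI_DamageTriggerInterpolated at an offset from the actor's bounds origin.
; Repair destroys that zone and the particle component, then swaps the mesh again.
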(fn ChangeMesh
  (params (OldMesh :type Static%20Mesh%20Component%20Object%20Reference) (NewMeshToSelect :type Array%20of%20Static%20Mesh%20Object%20References))
  (LocalVariables|SetOldMeshVar OldMesh)
  (LocalVariables|SetNewMeshToPick NewMeshToSelect)
  (if (== (Utilities|Array|Length (LocalVariables|GetNewMeshToPick)) 0)
    (return)
    (else
      (if (== (Utilities|Array|Length (LocalVariables|GetNewMeshToPick)) 1)
        (bind _returnvalue (Components|StaticMesh|SetStaticMesh (LocalVariables|GetOldMeshVar) (Utilities|Array|Get(acopy) (LocalVariables|GetNewMeshToPick))))
        (if _returnvalue
          _
          (else
            (Development|PrintString "Failed to Change Mesh" :!label _label)
            (return)))
        (else
          (bind _returnvalue_2 (Components|StaticMesh|SetStaticMesh (LocalVariables|GetOldMeshVar) (Utilities|Array|Get(acopy) (LocalVariables|GetNewMeshToPick) (Math|Random|RandomInteger (- (Utilities|Array|Length (LocalVariables|GetNewMeshToPick)) 1)))))
          (if _returnvalue_2
            _
            (else
              (goto _label)))))
      (return))))

(fn InitializeParticles
  (params (NiagaraSystem :type Niagara%20System%20Object%20Reference) (StaticMeshTarget :type Static%20Mesh%20Component%20Object%20Reference) (Actor :type Actor%20Object%20Reference))
  (bind _returnvalue (Niagara|SpawnSystemAttached NiagaraSystem (Variables|/Script/Engine.Actor|GetRootComponent Actor) "None" (/ (.Max (Components|StaticMesh|GetLocalBounds StaticMeshTarget)) 2.0) (Math|Rotator|MakeRotator -9e+01 0.0 0.0) "SnapToTarget" false false))
  (bind _output_get (Variables|Default|SetNiagara%20System _returnvalue))
  (return _output_get))

(fn Repair?
  (params (OldMesh :type Static%20Mesh%20Component%20Object%20Reference) (NewMeshToSelect :type Array%20of%20Static%20Mesh%20Object%20References))
  (Actor|DestroyActor (Variables|Default|GetDamageZone))
  (Components|DestroyComponent (Variables|Default|GetNiagara%20System))
  (CallFunction|ChangeMesh OldMesh NewMeshToSelect))

(fn BreakItem
  (params (NewMeshToSelect :type Array%20of%20Static%20Mesh%20Object%20References) (MeshComponent :type Static%20Mesh%20Component%20Object%20Reference) (NiagaraSystem :type Niagara%20System%20Object%20Reference) (Actor :type Actor%20Object%20Reference))
  (CallFunction|ChangeMesh MeshComponent NewMeshToSelect)
  (bind _returnvalue (CallFunction|InitializeParticles NiagaraSystem MeshComponent Actor))
  (return _returnvalue))

(fn SpawnDamagingZone
  (params (Actor :type Actor%20Object%20Reference) (LocationOffset :type Vector) (Scale :type Vector) (NiagaraSystem :type Niagara%20Component%20Object%20Reference))
  (bind _output_get (LocalVariables|SetTempActor Actor))
  (bind _output_get_2 (LocalVariables|SetTempTransform (Transformation|GetActorTransform _output_get)))
  (bind _returnvalue (Game|SpawnActorfromClass "/Game/Blueprints/Controllers/BPI_DamageTriggerInterpolated.BPI_DamageTriggerInterpolated_C" (Math|Transform|MakeTransform (+ (Math|Transform|TransformDirection _output_get_2 LocationOffset) (.Origin (Collision|GetActorBounds (LocalVariables|GetTempActor) true false)))) "AlwaysSpawn" "OverrideRootScale" 0 NiagaraSystem Scale 0))
  (bind _output_get_3 (Variables|Default|SetDamageZone _returnvalue))
  (Transformation|AttachActorToActor _output_get_3 0 "None" "KeepWorld" "KeepWorld" "KeepWorld" true))