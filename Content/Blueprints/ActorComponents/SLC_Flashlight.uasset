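; SLC_Flashlight is a light component that gives its owning actor a toggleable, camera-mounted flashlight.
; On BeginPlay it adds the flashlight input mapping context and attaches itself to the owner's camera.
; The input action flip-flops visibility with a switch sound, only for owners implementing BPI_Tools.
; That interface makes tools exclusive: the light reports its use to the owner and cannot switch on while another tool is active.
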(event Input|EnhancedActionEvents|EnhancedInputActionIA_Flashlight
  (params (ActionValue :type Boolean) (ElapsedSeconds :type Float%20%28double-precision%29) (TriggeredSeconds :type Float%20%28double-precision%29) (InputAction :type Input%20Action%20Object%20Reference :default "/Game/Input/Actions/IA_Flashlight.IA_Flashlight"))
  (bind _returnvalue (Components|GetOwner))
  (if (Utilities|DoesObjectImplementInterface _returnvalue "/Game/Blueprints/Interfaces/BPI_Tools.BPI_Tools_C")
    (if (Variables|Default|GetBeingUsed?)
      (bind _isa (Utilities|FlowControl|FlipFlop :!label _label)
        (:A
          _)
        (:B
          _))
      (Rendering|SetVisibility _isa false)
      (Audio|PlaySound2D "/Engine/VREditor/Sounds/UI/Flashlight_Switch.Flashlight_Switch" 1.0 1.0 0.0 0 0)
      (bind _output_get (Variables|Default|SetBeingUsed? _isa))
      (Class|BPITools|UsingTool(Message) _returnvalue _output_get)
      (else
        (bind _condition_ (Class|BPITools|IsUsingTool?(Message) _returnvalue))
        (if (not _condition_)
          (goto _label))))))

(event EventBeginPlay
  (Input|AddMappingContext (PlayerController|LocalPlayerSubsystems|GetEnhancedInputLocalPlayerSubsystem (Game|GetPlayerController 0)) "/Game/Input/IMC_Flashlight.IMC_Flashlight" 0 "(bIgnoreAllPressedKeysUntilRelease=True,bForceImmediately=False,bNotifyUserSettings=False)")
  (Transformation|AttachComponentToComponent (Actor|GetComponentbyClass (Components|GetOwner) "/Script/Engine.CameraComponent") "None" "KeepRelative" "KeepRelative" "KeepRelative" true))