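; Master door Blueprint that swings its Door component open or closed when InteractionResult fires.
; A Timeline drives the door's relative yaw from its DoorOpening track, playing from start to open and reversing to close.
; IsOpening blocks interaction while the door moves, and a FlipFlop on Finished toggles IsOpen to choose the next direction.
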(event EventInteractionResult
  (params (Player :type Actor%20Object%20Reference))
  (if (not (Variables|Default|GetIsOpening?))
    (if (not (Variables|Default|GetIsOpen?))
      (bind _dooropening (Timeline|Timeline PlayFromStart)
        (:Update
          (Variables|Default|SetIsOpening? true)
          (Transformation|SetRelativeRotation (Variables|Default|GetDoor) (Math|Rotator|MakeRotator 0.0 0.0 _dooropening) false false))
        (:Finished
          (bind _isa (Utilities|FlowControl|FlipFlop)
            (:A
              _)
            (:B
              _))
          (Variables|Default|SetIsOpen? _isa)
          (Variables|Default|SetIsOpening? false)))
      (else
        (Timeline|Timeline Reverse)))))

(fn ConstructionScript)