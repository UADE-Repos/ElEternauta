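; BP_Drawers is a furniture drawer that slides open and closed when it receives an interaction result.
; A timeline plays or reverses to lerp the static mesh's relative Y location from zero to AmountToOpen.
; IsOpening blocks interaction while the drawer moves, and a FlipFlop on timeline completion toggles IsOpen to choose the next direction.
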(event EventInteractionResult
  (params (Player :type Actor%20Object%20Reference))
  (if (not (Variables|Default|GetIsOpening?))
    (if (not (Variables|Default|GetIsOpen?))
      (bind _timetoopen (Timeline|Timeline Play)
        (:Update
          (Variables|Default|SetIsOpening? true)
          (Transformation|SetRelativeLocation (Variables|Default|GetStaticMesh) (Math|Vector|MakeVector 0.0 (Math|Float|Lerp 0.0 (Variables|Default|GetAmountToOpen) _timetoopen) 0.0) false false))
        (:Finished
          (bind _isa (Utilities|FlowControl|FlipFlop)
            (:A
              _)
            (:B
              _))
          (Variables|Default|SetIsOpen? _isa)
          (Variables|Default|SetIsOpening? false)))
      (else
        (Timeline|Timeline Reverse)))))

(fn ConstructionScript)