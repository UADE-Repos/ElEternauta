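; Base furniture light Blueprint that a linked light switch can turn on and off.
; The construction script applies the configured intensity and attenuation radius to the point light.
; BeginPlay creates a dynamic material for the chosen mesh slot and binds to the switch's TurnOnOff dispatcher, if a switch is valid.
; Toggling sets the material's Emission parameter and light intensity together, to configured amounts or zero.
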(event Custom|On/Off
  (params (Emission :type Float%20%28single-precision%29) (Intensity :type Float%20%28single-precision%29))
  (Rendering|Material|SetScalarParameterValue (Variables|Default|GetLightDynamicMaterial) "Emission" Emission :!class /Script/Engine.MaterialInstanceDynamic)
  (Rendering|Components|Light|SetIntensity (Variables|Default|GetPointLight) Intensity))

(event Custom|TurnOn/Off_Event
  (params (IsOn? :type Boolean))
  (if IsOn?
    (CallFunction|On/Off (Variables|Default|GetAmountOfEmission) (Variables|Default|GetAmountOfIntensity))
    (else
      (CallFunction|On/Off 0.0 0.0))))

(event EventBeginPlay
  (bind _lightmaterialindex (Variables|Default|GetLightMaterialIndex))
  (bind _lightswitchcall (Variables|Default|GetLightSwitchCall))
  (Utilities|FlowControl|Sequence
    (:then_0
      (bind _returnvalue (Rendering|Material|CreateDynamicMaterialInstance (Rendering|Material|GetMaterial (Variables|Default|GetLightMesh) _lightmaterialindex) "None" "None" :!class /Script/Engine.KismetMaterialLibrary))
      (bind _output_get (Variables|Default|SetLightDynamicMaterial _returnvalue))
      (Rendering|Material|SetMaterial (Variables|Default|GetLightMesh) _lightmaterialindex _output_get))
    (:then_1
      (Utilities|IsValid _lightswitchcall
        (:Is%20Valid
          (EventDispatchers|AssignTurnOn/Off _lightswitchcall (delegate Custom|TurnOn/Off_Event)))))))

(fn ConstructionScript
  (Rendering|Components|Light|SetIntensity (Variables|Default|GetPointLight) (Variables|Default|GetAmountOfIntensity))
  (Rendering|Lighting|SetAttenuationRadius (Variables|Default|GetPointLight) (Variables|Default|GetAmountOfAtenuation)))