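; BP_ObjectWithDissasemble is an interactable actor that breaks down into dropped objects.
; On BeginPlay it fits its Box collision to the mesh bounds.
; DoInteractionResult asks its AC_ObjectDissassemble component to spawn drops for its DisassemblableType at the actor's bounds center, then destroys the actor; without that component, nothing happens.
; IsHoveringActor returns an empty string.
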(event EventBeginPlay
  (CallFunction|CollisionSizeandLocation))

(event EventDoInteractionResult
  (params (HitResult :type Hit%20Result%20Structure))
  (bind _returnvalue (Actor|GetComponentbyClass "/Game/Blueprints/ActorComponents/AC_ObjectDissassemble.AC_ObjectDissassemble_C"))
  (Utilities|IsValid _returnvalue
    (:Is%20Valid
      (Class|BPISpawnerInterface|SpawnDroppedObjects(Message) _returnvalue (Variables|Default|GetDisassemblableType) (.Origin (Collision|GetActorBounds false false)))
      (Actor|DestroyActor))))

(fn ConstructionScript)

(fn CollisionSizeandLocation
  (bind _mesh (Variables|Default|GetMesh))
  (bind (_origin _boxextent) (Collision|GetComponentBounds _mesh))
  (Transformation|SetWorldLocation (Variables|Default|GetBox) _origin false false)
  (Components|Box|SetBoxExtent (Variables|Default|GetBox) _boxextent true))

(fn IsHoveringActor
  (params (Hit :type Hit%20Result%20Structure))
  (return ""))