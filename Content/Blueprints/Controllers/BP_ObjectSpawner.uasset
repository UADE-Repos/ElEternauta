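; BP_ObjectSpawner scatters dropped objects around a location based on a disassemble type.
; SpawnDroppedObjects uses the enum as a DTDisassembleObjects row name, then loops over ObjectTypes and Quantities, spawning BP_ObjectsToDrop with each type and matching mesh.
; GetPointInRadious randomizes X and Y with independent angle and distance rolls up to SpawnRadious, keeping Z.
; Debug prints remain, and the printed point is rolled separately from the spawn point.
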(event EventSpawnDroppedObjects
  (params (TypeOfDisassemble :type E_DisassemblableType%20Enum :default "NewEnumerator7") (SpawnLocation :type Vector :default "0, 0, 0"))
  (bind _locationselected (CallFunction|GetPointinRadious SpawnLocation))
  (bind _returnvalue (Utilities|GetDataTableRow (Variables|Default|GetDT_DisassembleObjects) (Utilities|String|StringToName (Utilities|String|EnumtoString TypeOfDisassemble)))
    (:then
      (for (_array_element _array_index) (.ObjectTypes (Utilities|Struct|BreakS_ItemToDrop _returnvalue))
        (for _array_element_2 (.Quantities (Utilities|Struct|BreakS_ItemToDrop _returnvalue))
          (Development|PrintString (Utilities|String|ToString(Vector) _locationselected))
          (Game|SpawnActorfromClass "/Game/Blueprints/BP_ObjectsToDrop.BP_ObjectsToDrop_C" (Math|Transform|MakeTransform _locationselected) "AlwaysSpawn" "MultiplyWithRoot" 0 (Utilities|Array|Get(acopy) (.ObjectMesh (Utilities|Struct|BreakS_ItemToDrop _returnvalue)) _array_index) _array_element 0))))
    (:RowNotFound
      (Development|PrintString "Hello"))))

(event EventBeginPlay
  (bind _outrownames (DataTable|GetDataTableRowNames (Variables|Default|GetDT_DisassembleObjects)))
  (Variables|Default|SetOut%20Row%20Names _outrownames))

(fn ConstructionScript)

(fn GetPointinRadious
  (params (Location :type Vector))
  (bind (_x _y _z) (Math|Vector|BreakVector Location))
  (bind _returnvalue (Math|Random|RandomFloatinRange 0.0 359.0))
  (bind _spawnradious (Variables|Default|GetSpawnRadious))
  (bind _returnvalue_2 (Math|Random|RandomFloatinRange 0.0 _spawnradious))
  (return (Math|Vector|MakeVector (+ (* (Math|Trig|Cos(Degrees) _returnvalue) _returnvalue_2) _x) (+ (* (Math|Trig|Sin(Degrees) _returnvalue) _returnvalue_2) _y) _z)))