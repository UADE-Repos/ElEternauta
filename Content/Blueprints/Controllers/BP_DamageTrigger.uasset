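; BP_DamageTrigger is a trigger that deals repeated damage to overlapping actors implementing BPI_SnowDamage.
; Begin overlap starts a looping 0.05-second timer that calls StartDamaging, which sends DoDamageMessage with AmountOfDamage to OtherActor.
; End overlap by an implementing actor clears the timer through the single stored DamagerHandle, so actors are not tracked individually.
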(event OnComponentBeginOverlap(DamageTrigger)
  (params (OverlappedComponent :type Primitive%20Component%20Object%20Reference) (OtherActor :type Actor%20Object%20Reference) (OtherComp :type Primitive%20Component%20Object%20Reference) (OtherBodyIndex :type Integer) (bFromSweep :type Boolean) (SweepResult :type Hit%20Result%20Structure%20%28by%20ref%29))
  (if (Utilities|DoesObjectImplementInterface OtherActor "/Game/Blueprints/Interfaces/BPI_SnowDamage.BPI_SnowDamage_C")
    (bind _returnvalue (Utilities|Time|SetTimerbyFunctionName 0 "StartDamaging" 0.05 true))
    (Variables|Default|SetDamagerHandle _returnvalue)))

(event OnComponentEndOverlap(DamageTrigger)
  (params (OverlappedComponent :type Primitive%20Component%20Object%20Reference) (OtherActor :type Actor%20Object%20Reference) (OtherComp :type Primitive%20Component%20Object%20Reference) (OtherBodyIndex :type Integer))
  (if (Utilities|DoesObjectImplementInterface OtherActor "/Game/Blueprints/Interfaces/BPI_SnowDamage.BPI_SnowDamage_C")
    (Utilities|Time|ClearandInvalidateTimerbyHandle (Variables|Default|GetDamagerHandle))))

(event Custom|StartDamaging
  (Class|BPISnowDamage|DoDamage(Message) (stale OnComponentBeginOverlap(DamageTrigger) OtherActor) (Variables|Default|GetAmountOfDamage)))

(fn ConstructionScript)