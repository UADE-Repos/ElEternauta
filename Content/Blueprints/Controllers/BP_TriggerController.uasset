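; Boundary trigger actor that toggles player damage and fog distance according to which side of the boundary is entered.
; Overlaps with the Inside and Outside components record the position status, and ending overlap with TriggerController evaluates it.
; Outside calls the dispatchers to start damage and decrease fog distance, while Inside calls those to stop damage and increase it.
; Overlaps are not filtered by actor, and debug prints remain.
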(event OnComponentBeginOverlap(Inside)
  (params (OverlappedComponent :type Primitive%20Component%20Object%20Reference) (OtherActor :type Actor%20Object%20Reference) (OtherComp :type Primitive%20Component%20Object%20Reference) (OtherBodyIndex :type Integer) (bFromSweep :type Boolean) (SweepResult :type Hit%20Result%20Structure%20%28by%20ref%29))
  (Variables|Default|SetPlayerPositionStatus "NewEnumerator1")
  (Development|PrintString (Utilities|String|EnumtoString (Variables|Default|GetPlayerPositionStatus))))

(event OnComponentBeginOverlap(Outside)
  (params (OverlappedComponent :type Primitive%20Component%20Object%20Reference) (OtherActor :type Actor%20Object%20Reference) (OtherComp :type Primitive%20Component%20Object%20Reference) (OtherBodyIndex :type Integer) (bFromSweep :type Boolean) (SweepResult :type Hit%20Result%20Structure%20%28by%20ref%29))
  (Variables|Default|SetPlayerPositionStatus "NewEnumerator0")
  (Development|PrintString (Utilities|String|EnumtoString (Variables|Default|GetPlayerPositionStatus))))

(event OnComponentEndOverlap(TriggerController)
  (params (OverlappedComponent :type Primitive%20Component%20Object%20Reference) (OtherActor :type Actor%20Object%20Reference) (OtherComp :type Primitive%20Component%20Object%20Reference) (OtherBodyIndex :type Integer))
  (CallFunction|CheckPlayerState)
  (Development|PrintString "Hello"))

(event Custom|CheckPlayerState
  (switch Utilities|FlowControl|Switch|SwitchonE_PlayerLocation (Variables|Default|GetPlayerPositionStatus)
    (:NewEnumerator0
      (Default|CallStartDamagePlayer)
      (Default|CallDecreaseFogDistance))
    (:NewEnumerator1
      (Default|CallStopDamagePlayer)
      (Default|CallIncreaseFogDistance))))

(fn ConstructionScript)