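; Controller that tracks every BP_BreakableWindow in the level and triggers random bursts of window destruction.
; On BeginPlay it sorts windows into available and broken lists, binding break and repair events only on the initially intact ones.
; Those events move windows between the lists, and a repair also calls WindowRepaired.
; DestructionRandomEvent starts destruction on randomly picked available windows, repeating a random number of times within configurable bounds.
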(event Custom|WindowHasBroken
  (params (Window :type BP%20Breakable%20Window%20Object%20Reference))
  (bind _windowsavailabletobreak (Variables|Default|GetWindowsAvailableToBreak))
  (if (Utilities|Array|ContainsItem _windowsavailabletobreak Window)
    (bind _returnvalue (Utilities|Array|RemoveItem _windowsavailabletobreak Window))
    (if _returnvalue
      (Utilities|Array|Add (Variables|Default|GetWindowsBroken) Window))))

(event Custom|DestructionRandomEvent
  (for _index (range 0 (- (Math|Random|RandomIntegerinRange (Variables|Default|GetMinToBreak) (Variables|Default|GetMaxToBreak)) 1))
    (CallFunction|WindowstoBreakRandom))
  (Development|PrintString "DoneBreaking"))

(event Custom|WindowsToBreakRandom
  (bind _windowsavailabletobreak (Variables|Default|GetWindowsAvailableToBreak))
  (Default|StartDestruction (Utilities|Array|Get(acopy) _windowsavailabletobreak (Math|Random|RandomInteger (- (Utilities|Array|Length _windowsavailabletobreak) 1)))))

(event Custom|GetAvailableWindows
  (for _array_element (Variables|Default|GetWindows)
    (if (Variables|/Game/Blueprints/Interactables/Furniture/BP_BreakableWindow.BP_BreakableWindow_C|GetAlreadyBroken? _array_element)
      (Utilities|Array|Add (Variables|Default|GetWindowsBroken) _array_element)
      (else
        (Utilities|Array|Add (Variables|Default|GetWindowsAvailableToBreak) _array_element)
        (EventDispatchers|BindEventtoWindowHasBroken _array_element (delegate Custom|WindowHasBroken))
        (EventDispatchers|BindEventtoWindowHasRepaired _array_element (delegate Custom|WindowHasRepaired))))))

(event Custom|WindowHasRepaired
  (params (Window :type BP%20Breakable%20Window%20Object%20Reference))
  (bind _windowsbroken (Variables|Default|GetWindowsBroken))
  (bind _windowsavailabletobreak (Variables|Default|GetWindowsAvailableToBreak))
  (if (Utilities|Array|ContainsItem _windowsbroken Window)
    (bind _returnvalue (Utilities|Array|RemoveItem _windowsbroken Window))
    (if _returnvalue
      (Utilities|Array|Add _windowsavailabletobreak Window)
      (Development|PrintString (Utilities|String|ToString(Integer) (Utilities|Array|Length _windowsavailabletobreak)))
      (Development|PrintString (Utilities|String|ToString(Integer) (Utilities|Array|Length _windowsbroken)))
      (Default|CallWindowRepaired))))

(event EventBeginPlay
  (bind _outactors (Actor|GetAllActorsOfClass "/Game/Blueprints/Interactables/Furniture/BP_BreakableWindow.BP_BreakableWindow_C"))
  (Variables|Default|SetWindows _outactors)
  (CallFunction|GetAvailableWindows))

(fn ConstructionScript)