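; BP_SnowSafeZones is a safe zone that shields actors from a configured snow damage type while they are inside its DamageTrigger.
; On overlap begin, it messages actors implementing BPI_SnowDamage to stop that damage and add invulnerability to it.
; On overlap end, it removes the invulnerability through the same interface, without restarting the stopped damage.
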(event OnComponentBeginOverlap(DamageTrigger)
  (params (OverlappedComponent :type Primitive%20Component%20Object%20Reference) (OtherActor :type Actor%20Object%20Reference) (OtherComp :type Primitive%20Component%20Object%20Reference) (OtherBodyIndex :type Integer) (bFromSweep :type Boolean) (SweepResult :type Hit%20Result%20Structure%20%28by%20ref%29))
  (if (Utilities|DoesObjectImplementInterface OtherActor "/Game/Blueprints/Interfaces/BPI_SnowDamage.BPI_SnowDamage_C")
    (Class|BPISnowDamage|StopDamagewithType(Message) OtherActor (Variables|Default|GetDamageToAvoid))
    (Class|BPISnowDamage|AddInvulnerability(Message) OtherActor (Variables|Default|GetDamageToAvoid))))

(event OnComponentEndOverlap(DamageTrigger)
  (params (OverlappedComponent :type Primitive%20Component%20Object%20Reference) (OtherActor :type Actor%20Object%20Reference) (OtherComp :type Primitive%20Component%20Object%20Reference) (OtherBodyIndex :type Integer))
  (if (Utilities|DoesObjectImplementInterface OtherActor "/Game/Blueprints/Interfaces/BPI_SnowDamage.BPI_SnowDamage_C")
    (Class|BPISnowDamage|RemoveInvulnerability(Message) OtherActor (Variables|Default|GetDamageToAvoid))))

(fn ConstructionScript
  (|CallParentFunction))