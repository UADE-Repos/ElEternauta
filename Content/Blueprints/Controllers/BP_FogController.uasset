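; Fog controller Blueprint that thins and thickens the level's volumetric fog.
; On BeginPlay it caches the ExponentialHeightFog actor and sets its volumetric fog distance.
; DecreaseFog plays a timeline that lerps the fog's start distance outward and extinction scale down, while IncreaseFog reverses it.
; A GetPointInRadious helper offsets a location on XY, but its zero radius range returns the input unchanged.
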(event Custom|DecreaseFog
  (bind _fog (Timeline|Decrease/IncreaseFog Play)
    (:Update
      (Class|ExponentialHeightFogComponent|SetVolumetricFogStartDistance (Variables|/Script/Engine.ExponentialHeightFog|GetComponent (Variables|Default|GetFogController)) (Math|Float|Lerp 1e+01 1.9e+03 _fog))
      (Class|ExponentialHeightFogComponent|SetVolumetricFogExtinctionScale (Variables|/Script/Engine.ExponentialHeightFog|GetComponent (Variables|Default|GetFogController)) (Math|Float|Lerp 5e+01 3e+01 _fog)))))

(event Custom|IncreaseFog
  (bind _fog (Timeline|Decrease/IncreaseFog Reverse)
    (:Update
      (Class|ExponentialHeightFogComponent|SetVolumetricFogStartDistance (Variables|/Script/Engine.ExponentialHeightFog|GetComponent (Variables|Default|GetFogController)) (Math|Float|Lerp 1e+01 1.9e+03 _fog))
      (Class|ExponentialHeightFogComponent|SetVolumetricFogExtinctionScale (Variables|/Script/Engine.ExponentialHeightFog|GetComponent (Variables|Default|GetFogController)) (Math|Float|Lerp 5e+01 3e+01 _fog)))))

(event EventBeginPlay
  (bind _returnvalue (Actor|GetActorOfClass "/Script/Engine.ExponentialHeightFog"))
  (bind _output_get (Variables|Default|SetFogController _returnvalue))
  (Class|ExponentialHeightFogComponent|SetVolumetricFogDistance (Variables|/Script/Engine.ExponentialHeightFog|GetComponent _output_get) 2e+03))

(fn ConstructionScript)

(fn GetPointinRadious
  (params (Location :type Vector))
  (bind (_x _y _z) (Math|Vector|BreakVector Location))
  (bind _returnvalue (Math|Random|RandomFloatinRange 0.0 0.0))
  (bind _returnvalue_2 (Math|Random|RandomFloatinRange 0.0 359.0))
  (return (Math|Vector|MakeVector (+ (* (Math|Trig|Cos(Degrees) _returnvalue_2) _returnvalue) _x) (+ (* (Math|Trig|Sin(Degrees) _returnvalue_2) _returnvalue) _y) _z)))