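; BP_DamageTriggerInterpolated is a damage trigger that switches on and off at a regular interval, paired with a Niagara effect.
; BeginPlay applies an optional scale, starts a looping timer at DelayTime and passes that delay to Niagara as LoopDelay.
; Each tick of the timer flip-flops the trigger's overlap events and in-game visibility, nudging it one unit up or down, apparently to refresh overlaps.
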(event Custom|GenerateOverlap
  (params (IsA? :type Boolean))
  (bind _damagetrigger (Variables|Default|GetDamageTrigger))
  (Variables|/Script/Engine.PrimitiveComponent|SetbGenerateOverlapEvents _damagetrigger IsA?)
  (Development|SetHiddeninGame _damagetrigger (not IsA?) false))

(event Custom|InterpolationTrigger
  (bind _isa (Utilities|FlowControl|FlipFlop)
    (:A
      _)
    (:B
      _))
  (CallFunction|GenerateOverlap _isa)
  (if _isa
    (Transformation|AddRelativeLocation (Variables|Default|GetDamageTrigger) "0.000000,0.000000,1.000000" false false)
    (else
      (Transformation|AddRelativeLocation (Variables|Default|GetDamageTrigger) "0.000000,0.000000,-1.000000" false false))))

(event EventBeginPlay
  (bind _niagarasystem (Variables|Default|GetNiagaraSystem))
  (bind _scale (Variables|Default|GetScale))
  (|CallParentFunction)
  (Utilities|IsValid _niagarasystem
    (:Is%20Valid
      (Components|Activation|Activate _niagarasystem false))
    (:Is%20Not%20Valid
      (Development|PrintString "Fallo de niagara")))
  (Utilities|FlowControl|Sequence
    (:then_0
      (if (Utilities|Operators|NotEqual(!=) :A _scale)
        (Transformation|SetActorScale3D _scale)))
    (:then_1
      (Utilities|Time|SetTimerbyFunctionName 0 "InterpolationTrigger" (Variables|Default|GetDelayTime) true true)
      (Utilities|IsValid (Variables|Default|GetNiagaraSystem)
        (:Is%20Valid
          (Niagara|SetNiagaraVariable(Float) (Variables|Default|GetNiagaraSystem) "LoopDelay" (Variables|Default|GetDelayTime)))))))

(fn ConstructionScript
  (|CallParentFunction))