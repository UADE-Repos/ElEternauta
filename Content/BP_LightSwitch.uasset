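; Interactable light switch that animates a rocking toggle and calls turn on/off with its state.
; Interaction plays or reverses a timeline based on the current state, lerping switch pitch, with a guard against retriggering mid-animation.
; When the timeline finishes, it flips the state and calls turn on/off.
; BeginPlay applies the initial state and, if off, offsets the timeline's start time for reverse playback.
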(event Custom|LightSwitchAnim
  (bind _rotationswitch (Variables|Default|GetRotationSwitch))
  (if (not (Variables|Default|GetSwitching?))
    (Variables|Default|SetSwitching? true)
    (if (Variables|Default|GetisOn?)
      (bind _animswitch (Timeline|LightSwitchTimeline Play)
        (:Update
          (Transformation|SetRelativeRotation (Variables|Default|GetLightSwitch) (Math|Rotator|MakeRotator 0.0 (Math|Float|Lerp (* _rotationswitch -1.0) _rotationswitch _animswitch) 0.0) false false))
        (:Finished
          (Variables|Default|SetSwitching? false)
          (bind _output_get (Variables|Default|SetisOn? (not (Variables|Default|GetisOn?))))
          (Default|CallTurnOn/Off _output_get)))
      (else
        (Timeline|LightSwitchTimeline Reverse)))))

(event Custom|SetTimerReset
  (params (On? :type Boolean))
  (bind _rotationswitch (Variables|Default|GetRotationSwitch))
  (if (not On?)
    ;[0.15 0.15 0.15 0.5 9] Si se cambia tiempo en timeline, ajustar.
    (bind _output_get (Variables|Default|SetTempTime 0.1))
    (bind _animswitch (Timeline|LightSwitchTimeline SetNewTime)
      (:Update
        (Transformation|SetRelativeRotation (Variables|Default|GetLightSwitch) (Math|Rotator|MakeRotator 0.0 (Math|Float|Lerp (* _rotationswitch -1.0) _rotationswitch _animswitch) 0.0) false false))
      (:Finished
        (Variables|Default|SetSwitching? false)
        (bind _output_get_2 (Variables|Default|SetisOn? (not (Variables|Default|GetisOn?))))
        (Default|CallTurnOn/Off _output_get_2)))))

(event EventBeginPlay
  (bind _ison_ (Variables|Default|GetisOn?))
  (Default|CallTurnOn/Off _ison_)
  (CallFunction|SetTimerReset _ison_))

(event EventInteractionResult
  (params (Player :type Actor%20Object%20Reference))
  (CallFunction|LightSwitchAnim))

(fn ConstructionScript)